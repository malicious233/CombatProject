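; BP_FighterCharacter is the fighter character Blueprint, currently little more than setup.
; On BeginPlay it casts the skeletal mesh's anim instance to ABP_Fighter and stores it as AnimBP for later access.
; An unconnected test chain, which never runs, prints the current state and switches it to WALKING, then IDLE, with delays.
; Tick, overlap and the construction script are empty.
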(event `self.ReceiveBeginPlay`
  ;[1 1 1] Set accessible AnimBP variable
  (bind _asabp_fighter (cast `/Game/Assets/Fighter/Animations/ABP_Fighter` (`SkeletalMeshComponent.GetAnimInstance` (`self.SkeletalMesh`))))
  (set `self.AnimBP` _asabp_fighter))

(fn `UserConstructionScript`)